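; BP_BombermanCharacter is the playable character in a Bomberman game, identified by PlayerIndex.
; On BeginPlay it teleports to its tagged PlayerStart, applies a green or red material by index and caches its max speed.
; Movement functions feed world-axis input to CharacterMovement.
; PlaceBomb spawns BP_Bomb at the nearest grid cell with itself as Instigator, capped by an active-bomb count that OnBombDestroyed decrements.
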(event `self.ReceiveBeginPlay`
  (`self.SetInitialTransform`)
  (`self.SetColor`)
  (set `self.MaxSpeed` (`MovementComponent.GetMaxSpeed` (`self.CharacterMovement`))))

(event `self.ReceiveTick`
  (params (DeltaSeconds :type "Float (single-precision)")))

(fn `MoveForward`
  (params (AxisValue :type "Float (double-precision)"))
  (`PawnMovementComponent.AddInputVector` (`self.CharacterMovement`) (`KismetMathLibrary.MakeVector` AxisValue) false))

(fn `MoveRight`
  (params (AxisValue :type "Float (double-precision)"))
  (`PawnMovementComponent.AddInputVector` (`self.CharacterMovement`) (`KismetMathLibrary.MakeVector` 0.0 AxisValue) false))

(fn `OnBombDestroyed`
  (`/Engine/EditorBlueprintResources/StandardMacros.DecrementInt` (`self.NumCurrentActiveBombs`)))

(fn `PlaceBomb`
  (locals (X :type Integer) (Y :type Integer))
  (if (not (>= (`self.NumCurrentActiveBombs`) (`self.MaxNumOfActiveBombs`)))
    (bind (_outx _outy) (`/Game/Blueprints/HelperFunctions.GetNearestGridPositionForActor` self))
    (bind _location (`/Game/Blueprints/BP_Grid.GetPositionForGrid2DCoords` (`/Game/Blueprints/HelperFunctions.GetGrid`) _outx _outy))
    (`|SpawnActorFromClass` "/Game/Bomb/BP_Bomb.BP_Bomb_C" (`KismetMathLibrary.MakeTransform` _location) "Undefined" "OverrideRootScale" null (`self.BombTimeUntilExplosion`) (`KismetMathLibrary.MakeVector2D` (`KismetMathLibrary.Conv_IntToDouble` _outx) (`KismetMathLibrary.Conv_IntToDouble` _outy)) self)
    (`/Engine/EditorBlueprintResources/StandardMacros.IncrementInt` (`self.NumCurrentActiveBombs`))))

(fn `SetColor`
  (bind _mesh (`self.Mesh`))
  (switch `int` (`self.PlayerIndex`)
    (:`0`
      (`PrimitiveComponent.SetMaterial` _mesh 0 "/Game/Materials/MI_Green.MI_Green"))
    (:`1`
      (`PrimitiveComponent.SetMaterial` _mesh 0 "/Game/Materials/MI_Red.MI_Red"))))

(fn `SetInitialTransform`
  (bind _outactors (`GameplayStatics.GetAllActorsOfClass` "/Script/Engine.PlayerStart"))
  (for _array_element _outactors
    (if (== (`PlayerStart.PlayerStartTag` _array_element) (`KismetStringLibrary.Conv_StringToName` (`KismetStringLibrary.Concat_StrStr` "Player" (`KismetStringLibrary.Conv_IntToString` (`self.PlayerIndex`)))))
      (bind _output_get (set `self.SpawnLocation` (`self.GetTransform` _array_element)))
      (`self.K2_SetActorTransform` _output_get false true))))

(fn `UserConstructionScript`)