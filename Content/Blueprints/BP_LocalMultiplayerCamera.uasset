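; Shared camera for two-player local multiplayer that keeps its spring arm centred between both players' pawns.
; After a short delay at BeginPlay, it caches both pawns, its starting height and their initial separation.
; Each tick it eases the arm toward their offset midpoint at that height.
; Arm length interpolates between min and max as player distance ranges up to that initial separation, zooming with spread.
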(event `self.ReceiveBeginPlay`
  (bind (_returnvalue_x _returnvalue_y _returnvalue_z) (`KismetMathLibrary.BreakVector` (`self.K2_GetActorLocation`)))
  (bind (_returnvalue_x_2 _returnvalue_y_2) (`KismetMathLibrary.BreakVector` (`SceneComponent.K2_GetComponentLocation` (`self.SpringArm`))))
  (`KismetSystemLibrary.Delay` 0.2)
  (`|ExecutionSequence`
    (:`then_0`
      (set `self.Character1` (`Controller.K2_GetPawn` (`GameplayStatics.GetPlayerController` 0)))
      (set `self.Character2` (`Controller.K2_GetPawn` (`GameplayStatics.GetPlayerController` 1))))
    (:`then_1`
      (set `self.CameraYPos` _returnvalue_y_2)
      (set `self.CameraXPos` _returnvalue_x_2)
      (set `self.CameraStartPosition` (`KismetMathLibrary.MakeVector` 0.0 0.0 _returnvalue_z)))
    (:`then_2`
      (`self.ArePlayersValid`
        (:`true`
          (set `self.InitialDistance` (`self.GetDistanceTo` (`self.Character1`) (`self.Character2`))))))))

(event `self.ReceiveTick`
  (params (DeltaSeconds :type "Float (single-precision)"))
  (`self.CameraZoom`)
  (`self.SetCameraPos`))

(event `CameraZoom`
  (`self.ArePlayersValid`
    (:`true`
      (set `SpringArmComponent.TargetArmLength` (`KismetMathLibrary.FInterpTo` (`SpringArmComponent.TargetArmLength` (`self.SpringArm`)) (`KismetMathLibrary.MapRangeClamped` (`self.GetDistanceTo` (`self.Character1`) (`self.Character2`)) 0.0 (`self.InitialDistance`) (`self.MinSpringArm`) (`self.MaxSpringArm`)) (`GameplayStatics.GetWorldDeltaSeconds`) 5.0) (`self.SpringArm`)))))

(event `SetCameraPos`
  (bind (_camerastartposition_x _camerastartposition_y _camerastartposition_z) (`KismetMathLibrary.BreakVector` (`self.CameraStartPosition`)))
  (set `self.CameraXPos` (`KismetMathLibrary.FInterpTo` (`self.CameraXPos`) (- (.x (`self.GetCenterPoint`)) (`self.XOffset`)) (`GameplayStatics.GetWorldDeltaSeconds`) 15.0))
  (set `self.CameraYPos` (`KismetMathLibrary.FInterpTo` (`self.CameraYPos`) (- (.y (`self.GetCenterPoint`)) (`self.YOffset`)) (`GameplayStatics.GetWorldDeltaSeconds`) 15.0))
  (`SceneComponent.K2_SetWorldLocation` (`self.SpringArm`) (`KismetMathLibrary.MakeVector` (`self.CameraXPos`) (`self.CameraYPos`) _camerastartposition_z) false false))

(fn `GetCenterPoint`
  (returns (ReturnValue :type "Vector Structure"))
  (`self.ArePlayersValid`
    (:`true`
      (return (/ (+ (`self.K2_GetActorLocation` (`self.Character1`)) (`self.K2_GetActorLocation` (`self.Character2`))) (2.0 2.0 2.0))))))

(fn `UserConstructionScript`)