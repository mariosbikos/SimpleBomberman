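; Bomberman player character that places itself at its own start point and moves on the world axes.
; On BeginPlay it teleports to the PlayerStart tagged "Player" plus its PlayerIndex, then calls SetColor.
; MoveForward and MoveRight feed axis values to CharacterMovement as world X and Y input.
; SetColor switches on PlayerIndex but has no actions in any branch.
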(event `self.ReceiveBeginPlay`
  (`self.Spawn`)
  (`self.SetColor`))

(fn `MoveForward`
  (params (AxisValue :type "Float (double-precision)"))
  (`PawnMovementComponent.AddInputVector` (`self.CharacterMovement`) (`KismetMathLibrary.MakeVector` AxisValue) false))

(fn `MoveRight`
  (params (AxisValue :type "Float (double-precision)"))
  (`PawnMovementComponent.AddInputVector` (`self.CharacterMovement`) (`KismetMathLibrary.MakeVector` 0.0 AxisValue) false))

(fn `SetColor`
  (switch `int` (`self.PlayerIndex`)))

(fn `Spawn`
  (bind _outactors (`GameplayStatics.GetAllActorsOfClass` "/Script/Engine.PlayerStart"))
  (for _array_element _outactors
    (if (== (`PlayerStart.PlayerStartTag` _array_element) (`KismetStringLibrary.Conv_StringToName` (`KismetStringLibrary.Concat_StrStr` "Player" (`KismetStringLibrary.Conv_IntToString` (`self.PlayerIndex`)))))
      (bind _output_get (set `self.SpawnLocation` (`self.GetTransform` _array_element)))
      (`self.K2_SetActorTransform` _output_get false true))))

(fn `UserConstructionScript`)