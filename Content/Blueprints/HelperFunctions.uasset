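; Helper functions for a Bomberman game that expose the level grid and convert actor positions to grid coordinates.
; GetGrid casts the current game mode to BP_BombermanGameMode and returns its Grid.
; GetCoordsClosestToChar snaps an actor's X and Y location to the nearest 100-unit cell and writes the integer indices into by-ref parameters.
; It also prints those coordinates on screen as debug output.
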(fn `GetCoordsClosestToChar`
  (params (Actor :type "Actor Object Reference") (X :type "Integer (by ref)") (Y :type "Integer (by ref)"))
  (bind (_returnvalue_x _returnvalue_y) (`KismetMathLibrary.BreakVector` (`Actor.K2_GetActorLocation` Actor)))
  (bind _returnvalue (/ (`KismetMathLibrary.FTrunc` (`KismetMathLibrary.GridSnap_Float` _returnvalue_y 100.0)) 100))
  (bind _returnvalue_2 (/ (`KismetMathLibrary.FTrunc` (`KismetMathLibrary.GridSnap_Float` _returnvalue_x 100.0)) 100))
  (cast `/Game/Core/BP_BombermanGameMode` (`GameplayStatics.GetGameMode` null))
  (`|VariableSetRef` X _returnvalue_2)
  (`|VariableSetRef` Y _returnvalue)
  (`KismetSystemLibrary.PrintString` null (`KismetTextLibrary.Conv_TextToString` (`|FormatText` "{x} - {y}" _returnvalue_2 _returnvalue))))

(fn `GetGrid`
  (returns (Grid :type "/Game/Blueprints/BP_Grid Object Reference"))
  (bind _asbp_bomberman_game_mode (cast `/Game/Core/BP_BombermanGameMode` (`GameplayStatics.GetGameMode` null)))
  (return (`/Game/Core/BP_BombermanGameMode.Grid` _asbp_bomberman_game_mode)))