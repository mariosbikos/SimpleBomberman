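; BP_Grid is a grid helper Blueprint that tracks which actor occupies each cell and maps cells to locations.
; Actors live in a flattened ActorsGrid array, written and read through a 2D-to-1D index conversion that multiplies X by GridMaxX.
; The reverse conversion divides by GridMaxY, so the two match only when both dimensions are equal.
; Cell coordinates convert to locations at 100-unit spacing with zero Z.
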(fn `GetActorForGridPos`
  (params (X :type Integer) (Y :type Integer))
  (returns (Output :type "Actor Object Reference"))
  (return (`|GetArrayItem` (`self.ActorsGrid`) (`self.Grid2DTo1DCoords` X Y))))

(fn `GetLocationForGridCoords`
  (params (X :type Integer) (Y :type Integer))
  (returns (Location :type "Vector Structure"))
  (return (`KismetMathLibrary.MakeVector` (`KismetMathLibrary.Conv_IntToDouble` (* X 100)) (`KismetMathLibrary.Conv_IntToDouble` (* Y 100)))))

(fn `Grid1DTo2DCoords`
  (params (`1D` :type Integer) (X :type "Integer (by ref)") (Y :type "Integer (by ref)"))
  (bind _gridmaxy (`self.GridMaxY`))
  (`|VariableSetRef` X (/ `1D` _gridmaxy))
  (`|VariableSetRef` Y (mod `1D` _gridmaxy)))

(fn `Grid2DTo1DCoords`
  (params (X :type Integer) (Y :type Integer))
  (returns (`1D` :type Integer))
  (return (+ (* X (`self.GridMaxX`)) Y)))

(fn `SetActorToGridPos`
  (params (X :type Integer) (Y :type Integer) (Actor :type "Actor Object Reference"))
  (`KismetArrayLibrary.Array_Set` (`self.ActorsGrid`) (`self.Grid2DTo1DCoords` X Y) Actor true))