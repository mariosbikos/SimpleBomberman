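; Bomberman-style bomb that explodes on a timer unless flagged IsRemote, then frees the instigating character's bomb capacity and destroys itself.
; OnExplosion calls CreateExplosion along forward, backward, right and left.
; Each direction line-traces in 100-unit steps up to BlastStrength, stopping at static mesh actors.
; Unblocked steps spawn a BP_Explosion that is immediately destroyed, and destroy any BP_DestructibleTile hit.
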(event `self.ReceiveBeginPlay`
  (if (not (`self.IsRemote`))
    (bind _returnvalue (`KismetSystemLibrary.K2_SetTimerDelegate` (delegate `OnExplosion`) (`self.TimeUntilExplosion`)))
    (set `self.ExplosionTimer` _returnvalue)))

(event `OnExplosion`
  (bind _returnvalue (`self.GetActorForwardVector` self))
  (bind _returnvalue_2 (`self.GetActorRightVector` self))
  (`self.CreateExplosion` _returnvalue)
  (`self.CreateExplosion` (* _returnvalue -1.0))
  (`self.CreateExplosion` _returnvalue_2)
  (`self.CreateExplosion` (* _returnvalue_2 -1.0))
  ;[1 1 1] DESTROY BOMB AND DECREASE CURRENT CAPACITY FOR BOMBS OF PLAYER
  (bind _asbp_bomberman_character (cast `/Game/Bomberman/BP_BombermanCharacter` (`self.GetInstigator`)))
  (`/Game/Bomberman/BP_BombermanCharacter.DecreaseBombCapacity` _asbp_bomberman_character)
  (`self.K2_DestroyActor`))

(fn `CreateExplosion`
  (params (Direction :type "Vector Structure"))
  (bind _returnvalue (`self.K2_GetActorLocation`))
  (for _index (range 1 (+ (`self.BlastStrength`) 1))
    (bind _returnvalue_2 (+ _returnvalue (* (* Direction 100.0) _index)))
    (bind _outhit (`KismetSystemLibrary.LineTraceSingle` :`Start` _returnvalue :`End` _returnvalue_2 :`TraceChannel` "TraceTypeQuery1" :`DrawDebugType` "ForOneFrame"))
    (cast `StaticMeshActor` (`.HitActor` (`GameplayStatics.BreakHitResult` _outhit))
      (:`then`
        (break))
      (:`CastFailed`
        (bind _returnvalue_3 (`|SpawnActorFromClass` "/Game/Blueprints/BP_Explosion.BP_Explosion_C" (`KismetMathLibrary.MakeTransform` (`KismetMathLibrary.MakeVector` (.x _returnvalue_2) (.y _returnvalue_2))) "AlwaysSpawn" "OverrideRootScale" null null))
        (`self.K2_DestroyActor` _returnvalue_3)
        (bind _asbp_destructible_tile (cast `/Game/Blueprints/BP_DestructibleTile` (`.HitActor` (`GameplayStatics.BreakHitResult` _outhit))))
        (`self.K2_DestroyActor` _asbp_destructible_tile)))))

(fn `UserConstructionScript`)