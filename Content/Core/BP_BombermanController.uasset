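; Player controller for a two-player Bomberman game that routes movement input to the controlled Bomberman character.
; Separate P1 and P2 axis events each cast the controlled pawn to BP_BombermanCharacter and call its MoveForward or MoveRight.
; A PlayerIndex check on the character filters the input, so each pawn responds only to its own player's axes.
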(event `InputAxis|P1_MoveForward`
  (params (AxisValue :type "Float (single-precision)"))
  ;[1 1 1] PLAYER 1
  (bind _asbp_bomberman_character (cast `/Game/Blueprints/BP_BombermanCharacter` (`self.K2_GetPawn`)))
  (if (== (`/Game/Blueprints/BP_BombermanCharacter.PlayerIndex` _asbp_bomberman_character) 0)
    (`/Game/Blueprints/BP_BombermanCharacter.MoveForward` _asbp_bomberman_character AxisValue)))

(event `InputAxis|P1_MoveRight`
  (params (AxisValue :type "Float (single-precision)"))
  ;[1 1 1] PLAYER 1
  (bind _asbp_bomberman_character (cast `/Game/Blueprints/BP_BombermanCharacter` (`self.K2_GetPawn`)))
  (if (== (`/Game/Blueprints/BP_BombermanCharacter.PlayerIndex` _asbp_bomberman_character) 0)
    (`/Game/Blueprints/BP_BombermanCharacter.MoveRight` _asbp_bomberman_character AxisValue)))

(event `InputAxis|P2_MoveForward`
  (params (AxisValue :type "Float (single-precision)"))
  (bind _asbp_bomberman_character (cast `/Game/Blueprints/BP_BombermanCharacter` (`self.K2_GetPawn`)))
  (if (== (`/Game/Blueprints/BP_BombermanCharacter.PlayerIndex` _asbp_bomberman_character) 1)
    (`/Game/Blueprints/BP_BombermanCharacter.MoveForward` _asbp_bomberman_character AxisValue)))

(event `InputAxis|P2_MoveRight`
  (params (AxisValue :type "Float (single-precision)"))
  (bind _asbp_bomberman_character (cast `/Game/Blueprints/BP_BombermanCharacter` (`self.K2_GetPawn`)))
  (if (== (`/Game/Blueprints/BP_BombermanCharacter.PlayerIndex` _asbp_bomberman_character) 1)
    (`/Game/Blueprints/BP_BombermanCharacter.MoveRight` _asbp_bomberman_character AxisValue)))

(fn `UserConstructionScript`)