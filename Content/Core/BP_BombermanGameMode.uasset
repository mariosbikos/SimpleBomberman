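; Game mode for a Bomberman game that sets up local multiplayer characters when play begins.
; SpawnPlayers creates the extra players up to MaxPlayers, as player 0 already exists.
; It then replaces each player controller's valid pawn with a BP_BombermanCharacter spawned at the world origin, passing in the player index and possessing it.
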(event `self.ReceiveBeginPlay`
  (`self.SpawnPlayers`))

(fn `SpawnPlayers`
  (bind _returnvalue (- (`self.MaxPlayers`) 1))
  (for _index (range 1 (+ _returnvalue 1))
    ;[1 1 1] Creates extra players. 0 is already created
    (`GameplayStatics.CreatePlayer` _index))
  (for _index_2 (range (+ _returnvalue 1))
    (bind _returnvalue_2 (`GameplayStatics.GetPlayerController` _index_2))
    (bind _returnvalue_3 (`Controller.K2_GetPawn` _returnvalue_2))
    (`/Engine/EditorBlueprintResources/StandardMacros.IsValid` _returnvalue_3
      (:`Is Valid`
        (`self.K2_DestroyActor` _returnvalue_3)
        (bind _returnvalue_4 (`|SpawnActorFromClass` "/Game/Blueprints/BP_BombermanCharacter.BP_BombermanCharacter_C" (`KismetMathLibrary.MakeTransform` (0.0 0.0 0.0)) "AlwaysSpawn" "OverrideRootScale" null _index_2 null))
        (`Controller.Possess` _returnvalue_2 _returnvalue_4)))))

(fn `UserConstructionScript`)